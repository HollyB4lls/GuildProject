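; Arm machine gun Blueprint for the RBMK1 that handles start and stop fire requests, with no actual shooting logic yet.
; StartFire and StopFire use authority switches to forward remote calls to the server.
; StartFire sets WantsToFire, calls an empty CameraAim and prints a debug string.
; StopFire clears WantsToFire only when it is already false, so it never resets the flag.
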(event Custom|Server_StartFire
  (CallFunction|StartFire))

(event Custom|Server_StopFire
  (CallFunction|StopFire))

(fn ConstructionScript)

(fn StartFire
  (Networking|SwitchHasAuthority
    (:Authority
      _)
    (:Remote
      (CallFunction|ServerStartFire)))
  (if (not (Variables|Default|GetWantsToFire))
    (Variables|Default|SetWantsToFire true)
    (CallFunction|CameraAim)
    (Development|PrintString "Should be firing weapon?" true true "(R=0.270000,G=0.000000,B=0.002344,A=1.000000)")))

(fn StopFire
  (Networking|SwitchHasAuthority
    (:Authority
      _)
    (:Remote
      (CallFunction|ServerStopFire)))
  (if (not (Variables|Default|GetWantsToFire))
    (Variables|Default|SetWantsToFire false)))

(fn CameraAim)