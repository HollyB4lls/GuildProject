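; Multiplayer game instance Blueprint that wraps online session hosting, searching, joining and destruction in four custom events, with LAN mode off.
; Hosting creates a session, then opens Starter_map as a listen server through a console command.
; Searching requests a single result and stores it in SessionResults, whose first entry the join event uses without a validity check.
; Each event prints debug strings for its outcomes, except a successful search.
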(event Custom|JOINGame
  ;[1 1 1] Join
  (|JoinSession (Game|GetPlayerController 0) (Utilities|Array|Get(acopy) (Variables|Default|GetSessionResults))
    (:OnSuccess
      (Development|PrintString "Successfully joined to sesion"))
    (:OnFailure
      (Development|PrintString "Session join error"))))

(event Custom|DESTROYGame
  ;[1 1 1] Destroy
  (|DestroySession (Game|GetPlayerController 0)
    (:OnSuccess
      (Development|PrintString "Successfully destroyed"))
    (:OnFailure
      (Development|PrintString "Session destroy error"))))

(event Custom|HOSTGame
  (bind _returnvalue (Game|GetPlayerController 0))
  ;[1 1 1] Host
  (|Session _returnvalue 0 false
    (:OnSuccess
      (Development|ExecuteConsoleCommand "open Starter_map?listen" _returnvalue)
      (Development|PrintString "Session created"))
    (:OnFailure
      (Development|PrintString "Session create error"))))

(event Custom|SEARCHGame
  ;[1 1 1] Search
  (bind _results (|FindSessions (Game|GetPlayerController 0) 1 false)
    (:OnSuccess
      (Variables|Default|SetSessionResults _results))
    (:OnFailure
      (Development|PrintString "Sessions not found"))))